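; Game mode for the main game, handling match setup, player joins, map travel and shared limits.
; On BeginPlay the authority spawns the EventNotifier, SolarController and AIDirector actors, keeping references to the first two.
; After a short delay, PostLogin copies Modifiers from the game instance into each SwarmPlayerState.
; Helpers draw player colours randomly from a shrinking pool, disable highlighting at three highlighted monsters, and perform server travel.
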(event Custom|MapTravel
  (params (Map%20Name :type String))
  (Class|SwarmGameMode|ServerTravel Map%20Name))

(event EventCheckHighlight
  (if (>= (Variables|Default|GetMonstersHighlighted) 3)
    (Variables|Default|SetCanHighlight false)
    (else
      (Variables|Default|SetCanHighlight true))))

(event EventPostLogin
  (params (NewPlayer :type Player%20Controller%20Object%20Reference))
  (bind _asswarm_player_state (Utilities|Casting|CastToSwarmPlayerState (Variables|/Script/Engine.Controller|GetPlayerState NewPlayer)))
  (Utilities|FlowControl|Delay 0.5)
  (bind _asmy_game_instance (Utilities|Casting|CastToMyGameInstance (Game|GetGameInstance)))
  (Variables|/Game/Blueprints/SwarmPlayerState.SwarmPlayerState_C|SetModifiers _asswarm_player_state (Variables|/Game/Blueprints/MyGameInstance.MyGameInstance_C|GetModifiers _asmy_game_instance)))

(event EventBeginPlay
  (bind _returnvalue (Math|Transform|MakeTransform "0, 0, 0"))
  (Networking|SwitchHasAuthority
    (:Authority
      (bind _returnvalue_2 (Game|SpawnActorfromClass "/Game/Blueprints/EventNotifier/EventNotifier.EventNotifier_C" _returnvalue "AlwaysSpawn" 0 0))
      (Variables|Default|SetEventNotifier _returnvalue_2)
      (bind _returnvalue_3 (Game|SpawnActorfromClass "/Game/EventStuff/SolarPlant/SolarController.SolarController_C" _returnvalue "AlwaysSpawn" 0 0))
      (Variables|Default|SetSolarController _returnvalue_3)
      (Game|SpawnActorfromClass "/Game/Blueprints/AI/AIDirector.AIDirector_C" _returnvalue "AlwaysSpawn" 0 0)
      (Utilities|FlowControl|Sequence
        (:then_0
          _)))
    (:Remote
      _))
  (Utilities|FlowControl|Delay 0.2))

(fn ConstructionScript)

(fn RandomColour
  (params (Player%20Character :type Player%20Character%20Object%20Reference))
  (bind _availablecolours (Variables|Default|GetAvailableColours))
  (LocalVariables|SetTempColour (Math|Random|RandomIntegerinRange 0 (- (Utilities|Array|Length _availablecolours) 1)))
  (Default|SetColourServer Player%20Character (Utilities|Array|Get(acopy) _availablecolours (LocalVariables|GetTempColour)))
  (Utilities|Array|RemoveIndex _availablecolours (LocalVariables|GetTempColour)))