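; EventNotifier is a Blueprint that queues timed, colored text messages and shows them one at a time on the HUD.
; CreateEvent appends a message with a capped duration to the queue.
; On Tick, with authority only, UpdateQueue pops the oldest entry when none is active and starts it after a brief timer.
; StartEvent fills player 0's HUD widget, then a timer calls EndEvent to flag the widget and free the queue.
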(event `StartEvent`
  (bind (_message _time _color) (break `/Game/Blueprints/EventNotifier/EventInfo` (`self.CurrentEvent`)))
  ;[1 1 1] Start Event
  (bind _asgame_hud (cast `/Game/Blueprints/GameHUD` (`PlayerController.GetHUD` (`GameplayStatics.GetPlayerController` 0))))
  (bind _hudwidget (`/Game/Blueprints/GameHUD.HUDWidget` _asgame_hud))
  (set `/Game/Widgets/HUD_Widget.StartEvent` true _hudwidget)
  (bind _eventtext (`/Game/Widgets/HUD_Widget.EVENTTEXT` _hudwidget))
  (`TextBlock.SetText` _eventtext (`KismetTextLibrary.Conv_StringToText` _message))
  (`TextBlock.SetColorAndOpacity` _eventtext (make `SlateColor` _color))
  (`Widget.SetVisibility` _eventtext "Visible")
  (`KismetSystemLibrary.K2_SetTimer` null "EndEvent" _time))

(event `Create Event`
  (params (Message :type String) (Time :type "Float (double-precision)") (Color :type "LinearColor Structure"))
  ;[1 1 1] Create an Event
  (`KismetArrayLibrary.Array_Add` (`self.EventQueue`) (make `/Game/Blueprints/EventNotifier/EventInfo` Message (`KismetMathLibrary.FMin` Time 20.0) Color)))

(event `EndEvent`
  ;[1 1 1] End Event
  (bind _asgame_hud (cast `/Game/Blueprints/GameHUD` (`PlayerController.GetHUD` (`GameplayStatics.GetPlayerController` 0))))
  (set `/Game/Widgets/HUD_Widget.EndEvent` true (`/Game/Blueprints/GameHUD.HUDWidget` _asgame_hud))
  (set `self.EventActive` false))

(event `self.ReceiveTick`
  (params (DeltaSeconds :type "Float (single-precision)"))
  ;[1 1 1] Tick
  (`/Engine/EditorBlueprintResources/ActorMacros.Switch Has Authority`
    (:`Authority`
      (`self.UpdateQueue`))))

(event `UpdateQueue`
  (bind _eventqueue (`self.EventQueue`))
  ;[1 1 1] Update Queue
  (if (`self.EventActive`)
    _
    (elif (> (`KismetArrayLibrary.Array_Length` _eventqueue) 0)
      (set `self.CurrentEvent` (`KismetArrayLibrary.Array_Get` _eventqueue))
      (`KismetArrayLibrary.Array_Remove` _eventqueue)
      (`KismetSystemLibrary.K2_SetTimer` null "StartEvent" 0.2)
      (set `self.EventActive` true))))

(fn `UserConstructionScript`)