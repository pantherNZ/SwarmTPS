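; Weapon controller owned by a SwarmCharacter, managing its four-slot inventory and active weapon.
; Initialise maps four weapon choices to classes, spawns and stores them in slot order, sets their owner and totals carried weight.
; The default weapon becomes active on the mesh's Gun socket, falling back to Pistol for NONE; other slots stay unattached or empty.
; ResetMeleeArray clears the active sword's damaged-actor list.
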(event EventResetMeleeArray
  (bind _activeweapon (Variables|Default|GetActiveWeapon))
  (if (Variables|/Script/Swarm.BaseGun|GetIsMelee _activeweapon)
    (bind _assword (Utilities|Casting|CastToSword _activeweapon))
    (Utilities|Array|Clear (Variables|/Game/Blueprints/Weapons/Sword.Sword_C|GetDamagedActors _assword))))

(fn ConstructionScript)

(fn Initialise
  (params (Default%20Weapon :type EWeaponType%20Enum) (Secondary%20Weapon :type EWeaponType%20Enum) (Tertiary%20Weapon :type EWeaponType%20Enum) (Quaternity%20Weapon :type EWeaponType%20Enum))
  (bind _inventory (Variables|Default|GetInventory))
  (Variables|Default|SetCurrentWeight 0)
  (Utilities|FlowControl|Sequence
    (:then_0
      (switch Utilities|FlowControl|Switch|SwitchonEWeaponType Default%20Weapon
        (:EGT_PISTOL
          (LocalVariables|SetTemp%20Gun "/Game/Blueprints/Weapons/Pistol.Pistol_C" :!label _label))
        (:EGT_GRENADELAUNCHER
          (LocalVariables|SetTemp%20Gun "/Game/Blueprints/Weapons/GrenadeLauncher.GrenadeLauncher_C"))
        (:EGT_KATANA
          (LocalVariables|SetTemp%20Gun "/Game/Blueprints/Weapons/Sword.Sword_C"))
        (:EGT_RIFLE
          (LocalVariables|SetTemp%20Gun "/Game/Blueprints/Weapons/Rifle.Rifle_C"))
        (:EGT_NONE
          (goto _label)))
      (bind _returnvalue (Game|SpawnActorfromClass (LocalVariables|GetTemp%20Gun) (Math|Transform|MakeTransform "0, 0, 0") "AlwaysSpawn" 0 0))
      (bind _output_get (Variables|Default|SetActiveWeapon _returnvalue))
      (Utilities|Array|SetArrayElem _inventory 0 _returnvalue true)
      (bind _asswarm_character (Utilities|Casting|CastToSwarmCharacter (Components|GetOwner)))
      (Class|Actor|AttachRootComponentto _output_get (Variables|/Script/Engine.Character|GetMesh _asswarm_character) "Gun" "SnapToTargetIncludingScale" true)
      (Actor|SetOwner _returnvalue _asswarm_character)
      (Variables|Default|SetCurrentWeight (+ (Variables|Default|GetCurrentWeight) (Variables|/Script/Swarm.BaseGun|GetWeight _returnvalue))))
    (:then_1
      (switch Utilities|FlowControl|Switch|SwitchonEWeaponType Secondary%20Weapon
        (:EGT_PISTOL
          (LocalVariables|SetTemp%20Gun "/Game/Blueprints/Weapons/Pistol.Pistol_C")
          (bind _returnvalue_2 (Game|SpawnActorfromClass (LocalVariables|GetTemp%20Gun) (Math|Transform|MakeTransform "0, 0, 0") "AlwaysSpawn" 0 0 :!label _label_2))
          (Utilities|Array|SetArrayElem _inventory 1 _returnvalue_2 true)
          (bind _asswarm_character_2 (Utilities|Casting|CastToSwarmCharacter (Components|GetOwner)))
          (Actor|SetOwner _returnvalue_2 _asswarm_character_2)
          (Variables|Default|SetCurrentWeight (+ (Variables|/Script/Swarm.BaseGun|GetWeight _returnvalue_2) (Variables|Default|GetCurrentWeight))))
        (:EGT_GRENADELAUNCHER
          (LocalVariables|SetTemp%20Gun "/Game/Blueprints/Weapons/GrenadeLauncher.GrenadeLauncher_C")
          (goto _label_2))
        (:EGT_KATANA
          (LocalVariables|SetTemp%20Gun "/Game/Blueprints/Weapons/Sword.Sword_C")
          (goto _label_2))
        (:EGT_RIFLE
          (LocalVariables|SetTemp%20Gun "/Game/Blueprints/Weapons/Rifle.Rifle_C")
          (goto _label_2))
        (:EGT_NONE
          (Utilities|Array|SetArrayElem _inventory 1 0 true))))
    (:then_2
      (switch Utilities|FlowControl|Switch|SwitchonEWeaponType Tertiary%20Weapon
        (:EGT_PISTOL
          (LocalVariables|SetTemp%20Gun "/Game/Blueprints/Weapons/Pistol.Pistol_C")
          (bind _returnvalue_3 (Game|SpawnActorfromClass (LocalVariables|GetTemp%20Gun) (Math|Transform|MakeTransform "0, 0, 0" "0, 0, 0" "1.000000,1.000000,1.000000") "AlwaysSpawn" 0 0 :!label _label_3))
          (Utilities|Array|SetArrayElem _inventory 2 _returnvalue_3 true)
          (bind _asswarm_character_3 (Utilities|Casting|CastToSwarmCharacter (Components|GetOwner)))
          (Actor|SetOwner _returnvalue_3 _asswarm_character_3)
          (Variables|Default|SetCurrentWeight (+ (Variables|/Script/Swarm.BaseGun|GetWeight _returnvalue_3) (Variables|Default|GetCurrentWeight))))
        (:EGT_GRENADELAUNCHER
          (LocalVariables|SetTemp%20Gun "/Game/Blueprints/Weapons/GrenadeLauncher.GrenadeLauncher_C")
          (goto _label_3))
        (:EGT_KATANA
          (LocalVariables|SetTemp%20Gun "/Game/Blueprints/Weapons/Sword.Sword_C")
          (goto _label_3))
        (:EGT_RIFLE
          (LocalVariables|SetTemp%20Gun "/Game/Blueprints/Weapons/Rifle.Rifle_C")
          (goto _label_3))
        (:EGT_NONE
          (Utilities|Array|SetArrayElem _inventory 2 0 true))))
    (:then_3
      (switch Utilities|FlowControl|Switch|SwitchonEWeaponType Quaternity%20Weapon
        (:EGT_PISTOL
          (LocalVariables|SetTemp%20Gun "/Game/Blueprints/Weapons/Pistol.Pistol_C")
          (bind _returnvalue_4 (Game|SpawnActorfromClass (LocalVariables|GetTemp%20Gun) (Math|Transform|MakeTransform "0, 0, 0") "AlwaysSpawn" 0 0 :!label _label_4))
          (Utilities|Array|SetArrayElem _inventory 3 _returnvalue_4 true)
          (bind _asswarm_character_4 (Utilities|Casting|CastToSwarmCharacter (Components|GetOwner)))
          (Actor|SetOwner _returnvalue_4 _asswarm_character_4)
          (Variables|Default|SetCurrentWeight (+ (Variables|/Script/Swarm.BaseGun|GetWeight _returnvalue_4) (Variables|Default|GetCurrentWeight))))
        (:EGT_GRENADELAUNCHER
          (LocalVariables|SetTemp%20Gun "/Game/Blueprints/Weapons/GrenadeLauncher.GrenadeLauncher_C")
          (goto _label_4))
        (:EGT_KATANA
          (LocalVariables|SetTemp%20Gun "/Game/Blueprints/Weapons/Sword.Sword_C")
          (goto _label_4))
        (:EGT_RIFLE
          (LocalVariables|SetTemp%20Gun "/Game/Blueprints/Weapons/Rifle.Rifle_C")
          (goto _label_4))
        (:EGT_NONE
          (Utilities|Array|SetArrayElem _inventory 3 0 true))))))