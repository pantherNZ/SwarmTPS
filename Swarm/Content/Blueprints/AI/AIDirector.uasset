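; AI Director that spawns the wave's swarm enemies into the world by monster type.
; SpawnMonsterinWorld maps the type to an enemy class, also announcing Broodmother spawns through the game mode's event notifier.
; SpawnNewActor spawns the AI pawn, updates spawned and alive counts, and pops the last entry from the Monsters array.
; When few kills remain in the wave, it multicasts an outline on each newly spawned monster.
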(event `self.SpawnMonsterInWorld`
  (params (Location :type "Vector Structure") (Rotation :type "Rotator Structure") (Scale :type "Vector Structure") (Type :type "EMonsterType Enum" :default "EMT_SWARMER_SMALL"))
  (bind _returnvalue (`KismetMathLibrary.MakeTransform` Location Rotation (1.0 1.0 1.0)))
  (switch `EMonsterType` Type
    (:`EMT_SWARMER_SMALL`
      (`self.SpawnNewActor` "/Game/Blueprints/AI/Swarmer/Enemy_Swarmer_Small.Enemy_Swarmer_Small_C" _returnvalue true))
    (:`EMT_SWARMER_MEDIUM`
      (`self.SpawnNewActor` "/Game/Blueprints/AI/Swarmer/Enemy_Swarmer_Medium.Enemy_Swarmer_Medium_C" _returnvalue true))
    (:`EMT_SWARMER_LARGE`
      (`self.SpawnNewActor` "/Game/Blueprints/AI/Swarmer/Enemy_Swarmer_Large.Enemy_Swarmer_Large_C" _returnvalue true))
    (:`EMT_SLAMMER`
      (`self.SpawnNewActor` "/Game/Blueprints/AI/Slammer/Enemy_Slammer.Enemy_Slammer_C" _returnvalue true))
    (:`EMT_SPITTER`
      (`self.SpawnNewActor` "/Game/Blueprints/AI/Spitter/Enemy_Spitter.Enemy_Spitter_C" _returnvalue true))
    (:`EMT_BROODMOTHER`
      (`self.SpawnNewActor` "/Game/Blueprints/AI/Broodmother/Enemy_Broodmother.Enemy_Broodmother_C" _returnvalue true)
      (bind _asmain_game_mode (cast `/Game/Blueprints/MainGameMode` (`GameplayStatics.GetGameMode`)))
      (`/Game/Blueprints/EventNotifier/EventNotifier.Create Event` (`/Game/Blueprints/MainGameMode.EventNotifier` _asmain_game_mode) "A Broodmother has spawned!" 5.0 (struct :`R` 1.0 :`A` 1.0)))))

(fn `SpawnNewActor`
  (params (Class :type "BaseMonster Class Reference") (Transform :type "Transform Structure") (RemoveIndex :type Boolean))
  (returns (Monster :type "/Game/Blueprints/AI/SwarmMonster Object Reference"))
  (bind _monsters (`self.Monsters`))
  (bind _returnvalue (`AIBlueprintHelperLibrary.SpawnAIFromClass` Class null (.location Transform) (.rotation Transform) false null))
  (`/Engine/EditorBlueprintResources/StandardMacros.IsValid` _returnvalue
    (:`Is Valid`
      (bind _asswarm_game_state (cast `/Game/Blueprints/SwarmGameState` (`GameplayStatics.GetGameState`))
        (:`then`
          (`|ExecutionSequence`
            (:`then_0`
              (`/Engine/EditorBlueprintResources/StandardMacros.IncrementInt` (`self.MonstersSpawned`)
                (:`  `
                  (bind _result (`/Engine/EditorBlueprintResources/StandardMacros.IncrementInt` (`BaseGameState.MonstersAlive` _asswarm_game_state))
                    (:`  `
                      (if RemoveIndex
                        (`KismetArrayLibrary.Array_Remove` _monsters (`KismetArrayLibrary.Array_LastIndex` _monsters))))))))
            (:`then_1`
              (if (<= (- (`BaseGameState.MonstersMax` _asswarm_game_state) (`BaseGameState.CurrentWaveKills` _asswarm_game_state)) 7)
                (bind _asswarm_monster (cast `/Game/Blueprints/AI/SwarmMonster` _returnvalue))
                (`/Game/Blueprints/AI/SwarmMonster.MulticastRenderOutline` _asswarm_monster)))
            (:`then_2`
              (bind _asswarm_monster_2 (cast `/Game/Blueprints/AI/SwarmMonster` _returnvalue)
                (:`then`
                  (return _asswarm_monster_2))
                (:`CastFailed`
                  (return null))))))
        (:`CastFailed`
          (return null))))
    (:`Is Not Valid`
      (return null))))

(fn `UserConstructionScript`)