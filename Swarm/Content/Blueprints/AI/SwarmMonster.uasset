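; Swarm monster Blueprint that handles wave scaling, blood effects, highlighting and money payouts for AI enemies.
; On Initalise, the server picks green or purple blood and scales health and damage by wave and difficulty, randomly varying health.
; Multicasts spawn color-matched ground splats by chance and enable custom-depth outlines, whose timed removal updates the game mode's highlight count.
; Money is split evenly between all player states.
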(event `self.Initalise`
  (bind _decalmaterial (`self.DecalMaterial`))
  (bind _health (`self.Health`))
  (bind _damage (`self.Damage`))
  (bind _returnvalue (/ _health (`self.WaveDoubleStrength`)))
  (`|ExecutionSequence`
    (:`then_0`
      (`KismetArrayLibrary.Array_Add` _decalmaterial "/Game/Textures/Decals/Blood/AlienSplatGreen1.AlienSplatGreen1")
      (`KismetArrayLibrary.Array_Add` _decalmaterial "/Game/Textures/Decals/Blood/AlienSplatGreen2.AlienSplatGreen2")
      (`KismetArrayLibrary.Array_Add` _decalmaterial "/Game/Textures/Decals/Blood/AlienSplatPurple1.AlienSplatPurple1")
      (`KismetArrayLibrary.Array_Add` _decalmaterial "/Game/Textures/Decals/Blood/AlienSplatPurple2.AlienSplatPurple2"))
    (:`then_1`
      (`/Engine/EditorBlueprintResources/ActorMacros.Switch Has Authority`
        (:`Authority`
          (bind _asmy_game_instance (cast `/Game/Blueprints/MyGameInstance` (`GameplayStatics.GetGameInstance`)))
          (`|ExecutionSequence`
            (:`then_0`
              (if (`KismetMathLibrary.RandomBool`)
                (set `self.HitParticle` "/Game/Blood/BloodImpacts/GreenBlood.GreenBlood")
                (else
                  (set `self.HitParticle` "/Game/Blood/BloodImpacts/PurpleBlood.PurpleBlood"))))
            (:`then_1`
              (bind _asbase_game_state (cast `BaseGameState` (`GameplayStatics.GetGameState`)))
              (bind _wavenumber (`BaseGameState.WaveNumber` _asbase_game_state))
              (set `self.Health` (+ _health (`KismetMathLibrary.RandomFloatInRange` (- 0.0 _returnvalue) _returnvalue) (* _wavenumber (* _returnvalue (`/Game/Blueprints/MyGameInstance.DifficultyMultiplier` _asmy_game_instance)))))
              (set `self.Damage` (+ _damage (* _wavenumber (* (/ _damage (`self.WaveDoubleStrength`)) (`/Game/Blueprints/MyGameInstance.DifficultyMultiplier` _asmy_game_instance))))))))))))

(event `DecalMulticast`
  (params (Direction :type "Vector Structure"))
  (bind _returnvalue (`self.K2_GetActorLocation`))
  (bind _monstertype (`self.MonsterType`))
  (bind (_returnvalue_x _returnvalue_y) (`KismetMathLibrary.BreakVector` (`BoxComponent.GetScaledBoxExtent` (`self.Collision`))))
  (bind _returnvalue_2 (- (+ (* Direction 50.0) _returnvalue) (0.0 0.0 80.0)))
  (bind _returnvalue_3 (`KismetMathLibrary.MakeVector` _returnvalue_x _returnvalue_y 200.0))
  (bind _returnvalue_4 (`KismetMathLibrary.FindLookAtRotation` (- _returnvalue (0.0 0.0 40.0)) _returnvalue_2))
  (if (or (and (== (`KismetMathLibrary.RandomIntegerInRange` 0 4) 0) (`|EnumEquality` _monstertype "EMT_SLAMMER")) (and (== (`KismetMathLibrary.RandomIntegerInRange` 0 2) 0) (`|EnumInequality` _monstertype "EMT_SLAMMER")))
    (if (== (`self.HitParticle`) "/Game/Blood/BloodImpacts/GreenBlood.GreenBlood")
      (`GameplayStatics.SpawnDecalAtLocation` (`KismetArrayLibrary.Array_Get` (`self.DecalMaterial`) (`KismetMathLibrary.RandomIntegerInRange` 0 1)) _returnvalue_3 _returnvalue_2 _returnvalue_4 40.0) ; Ground Splatter
      (else
        (`GameplayStatics.SpawnDecalAtLocation` (`KismetArrayLibrary.Array_Get` (`self.DecalMaterial`) (`KismetMathLibrary.RandomIntegerInRange` 2 3)) _returnvalue_3 _returnvalue_2 _returnvalue_4 40.0) ; Ground Splatter
      ))))

(event `self.SpawnDecal`
  (params (Direction :type "Vector Structure"))
  (`self.DecalMulticast` Direction))

(event `self.ShowMonsterOutline`
  (`self.MulticastRenderOutline`))

(event `MulticastRenderOutline`
  (`PrimitiveComponent.SetRenderCustomDepth` (`self.Mesh`) true))

(event `self.ReceiveTick`
  (params (DeltaSeconds :type "Float (single-precision)"))
  (`parent.ReceiveTick` DeltaSeconds))

(event `self.CheckOutlineTimer`
  (bind _outlinetimer (`self.OutlineTimer`))
  (`/Engine/EditorBlueprintResources/ActorMacros.Switch Has Authority`
    (:`Authority`
      (bind _asmain_game_mode (cast `/Game/Blueprints/MainGameMode` (`GameplayStatics.GetGameMode`)))
      (set `SwarmGameMode.CanHighlight` false _asmain_game_mode)
      (if (`KismetSystemLibrary.K2_IsValidTimerHandle` _outlinetimer)
        (if (`KismetSystemLibrary.K2_IsTimerActiveHandle` _outlinetimer)
          (`KismetSystemLibrary.K2_ClearTimerHandle` _outlinetimer))))))

(event `self.GiveMoneyToPlayers`
  (params (Money :type "Float (single-precision)") (Location :type "Vector Structure"))
  (bind _playerarray (`GameState.PlayerArray` (`GameplayStatics.GetGameState`)))
  (for _array_element _playerarray
    (bind _asswarm_player_state (cast `/Game/Blueprints/SwarmPlayerState` _array_element))
    (`BasePlayerState.UpdateMoney` _asswarm_player_state (`KismetMathLibrary.Conv_IntToDouble` (`KismetMathLibrary.Round` (/ Money (`KismetMathLibrary.Conv_IntToDouble` (`KismetArrayLibrary.Array_Length` _playerarray))))) Location)))

(fn `DisableOutline`
  (`PrimitiveComponent.SetRenderCustomDepth` (`self.Mesh`) false)
  (set `self.OutlineTimer` (struct))
  (`/Engine/EditorBlueprintResources/ActorMacros.Switch Has Authority`
    (:`Authority`
      (bind _asmain_game_mode (cast `/Game/Blueprints/MainGameMode` (`GameplayStatics.GetGameMode`)))
      (`/Engine/EditorBlueprintResources/StandardMacros.DecrementInt` (`SwarmGameMode.MonstersHighlighted` _asmain_game_mode)
        (:`  `
          (`/Game/Blueprints/MainGameMode.CheckHighlight` _asmain_game_mode))))))

(fn `StartTimerDisable`
  (bind _returnvalue (`KismetSystemLibrary.K2_SetTimer` null "DisableOutline" 15.0))
  (set `self.OutlineTimer` _returnvalue))

(fn `ToggleOffTouching`)

(fn `UserConstructionScript`)