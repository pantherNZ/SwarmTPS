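; Base gib actor for monster remains that removes itself after a short lifespan.
; Construction copies the owning SwarmMonster's mesh material onto the carcass and pieces.
; ImpulseGib pushes a piece away from the owner's death position, or actor center without death strength, adding random lift and applying linear and angular impulses through a multicast event.
; ParticleSpawn scatters a random number of the owner's scaled hit particles around the actor.
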(event `/Game/Blueprints/AI/Swarmer/Gibs/Swarmer_Gibs_Small.ReceiveBeginPlay`
  (`self.SetLifeSpan` 10.0))

(event `ImpulseMulticast`
  (params (Force :type "Vector Structure") (Gib :type "StaticMeshComponent Object Reference"))
  (`PrimitiveComponent.AddImpulse` Gib Force "None" false)
  (`PrimitiveComponent.AddAngularImpulse` Gib Force "None" false))

(fn `ImpulseGib`
  (params (Gib :type "StaticMeshComponent Object Reference") (Multiplier :type "Float (double-precision)"))
  (bind _returnvalue (`SceneComponent.K2_GetComponentLocation` Gib))
  (bind _returnvalue_2 (`KismetMathLibrary.RandomFloatInRange` 0.5 1.0))
  (bind _returnvalue_3 (* (`self.Strength`) Multiplier))
  (bind _asbase_monster (cast `BaseMonster` (`self.GetOwner`)))
  (bind _deathstrength (`BaseMonster.DeathStrength` _asbase_monster))
  (if (!= _deathstrength 0.0)
    (`self.ImpulseMulticast` (* (+ (* (`KismetMathLibrary.Normal` (- _returnvalue (`BaseMonster.DeathPosition` _asbase_monster))) _deathstrength) (`KismetMathLibrary.MakeVector` 0.0 0.0 (* _returnvalue_2 _deathstrength))) _returnvalue_3) Gib)
    (else
      (`self.ImpulseMulticast` (* (+ (`KismetMathLibrary.Normal` (- _returnvalue (`self.K2_GetActorLocation`))) (`KismetMathLibrary.MakeVector` 0.0 0.0 _returnvalue_2)) _returnvalue_3) Gib))))

(fn `ParticleSpawn`
  (params (Scale :type "Float (double-precision)") (Spread :type "Float (double-precision)") (Min :type Integer) (Max :type Integer))
  (bind _asbase_monster (cast `BaseMonster` (`self.GetOwner`)))
  (for _ (range 1 (+ (`KismetMathLibrary.RandomIntegerInRange` Min Max) 1))
    (bind _returnvalue (`GameplayStatics.SpawnEmitterAtLocation` (`BaseMonster.HitParticle` _asbase_monster) (+ (`self.K2_GetActorLocation`) (* (`KismetMathLibrary.RandomUnitVector`) Spread))))
    (`/Engine/EditorBlueprintResources/StandardMacros.IsValid` _returnvalue
      (:`Is Valid`
        (`SceneComponent.SetWorldScale3D` _returnvalue (`KismetMathLibrary.MakeVector` Scale Scale Scale))))))

(fn `UserConstructionScript`
  (bind _asswarm_monster (cast `/Game/Blueprints/AI/SwarmMonster` (`self.GetOwner`)))
  (`|ExecutionSequence`
    (:`then_0`
      (bind _returnvalue (`PrimitiveComponent.GetMaterial` (`Character.Mesh` _asswarm_monster) 0))
      (`PrimitiveComponent.SetMaterial` (`self.Carcass`) 0 _returnvalue))
    (:`then_1`
      (`PrimitiveComponent.SetMaterial` (`self.StaticMesh1`) 0 _returnvalue))
    (:`then_2`
      (`PrimitiveComponent.SetMaterial` (`self.StaticMesh2`) 0 _returnvalue))
    (:`then_3`
      (`PrimitiveComponent.SetMaterial` (`self.StaticMesh3`) 0 _returnvalue))
    (:`then_4`
      (`PrimitiveComponent.SetMaterial` (`self.StaticMesh`) 0 _returnvalue))
    (:`then_5`
      (`PrimitiveComponent.SetMaterial` (`self.StaticMesh4`) 0 _returnvalue))
    (:`then_6`
      (`PrimitiveComponent.SetMaterial` (`self.StaticMesh8`) 0 _returnvalue))
    (:`then_7`
      (`PrimitiveComponent.SetMaterial` (`self.StaticMesh6`) 0 _returnvalue))
    (:`then_8`
      (`PrimitiveComponent.SetMaterial` (`self.StaticMesh5`) 0 _returnvalue))
    (:`then_9`
      (`PrimitiveComponent.SetMaterial` (`self.StaticMesh7`) 0 _returnvalue))))