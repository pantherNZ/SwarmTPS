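; JumpTrigger is an actor that makes SwarmMonster AI leap when they overlap it.
; On overlap, only the authority checks that the actor is a SwarmMonster and that the Jump flag is set.
; It then calls LaunchCharacter, adding a forward and upward velocity, both scaled by JumpHeight, to the monster's current velocity.
; A yaw-alignment check and a plain Jump call are left unused.
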(event `self.ReceiveActorBeginOverlap`
  (params (OtherActor :type "Actor Object Reference"))
  (bind _jumpheight (`self.JumpHeight`))
  (`/Engine/EditorBlueprintResources/ActorMacros.Switch Has Authority`
    (:`Authority`
      (bind _asswarm_monster (cast `/Game/Blueprints/AI/SwarmMonster` OtherActor))
      (if (`self.Jump`)
        (`Character.LaunchCharacter` _asswarm_monster (+ (* (`self.GetActorForwardVector` _asswarm_monster) _jumpheight) (`KismetMathLibrary.MakeVector` 0.0 0.0 _jumpheight)) false false)))))

(fn `UserConstructionScript`)