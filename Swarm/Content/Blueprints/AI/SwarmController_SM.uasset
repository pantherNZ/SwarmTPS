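; AI controller for swarm monsters that picks, chases and attacks players or the life support.
; The server gathers targets, and a randomised timer re-runs FindTarget, scoring players by reachability, distance, speed, battery carrying and health, plus random noise.
; When generator power is off, life support usually gets an overwhelming score.
; Helper functions handle chasing with a ground-trace fallback, validate targets and switch monster CHASING/ATTACKING state from attack-collision overlaps.
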(event EventBeginPlay
  (Networking|SwitchHasAuthority
    (:Authority
      (Utilities|FlowControl|Delay 0.1)
      (bind _outactors (Actor|GetAllActorsOfClass "/Game/Blueprints/PlayerCharacter.PlayerCharacter_C"))
      (bind _output_get (Variables|Default|SetTargetList _outactors))
      (bind _outactors_2 (Actor|GetAllActorsOfClass "/Game/EventStuff/LifeSupport/LifeSupportBP.LifeSupportBP_C"))
      (Utilities|Array|Add _output_get (Utilities|Array|Get(acopy) _outactors_2))
      (bind _outactors_3 (Actor|GetAllActorsOfClass "/Game/EventStuff/Generator/GeneratorBP.GeneratorBP_C"))
      (Variables|Default|SetGeneratorBP (Utilities|Array|Get(acopy) _outactors_3))
      (CallFunction|FindTarget)
      (bind _returnvalue (Utilities|Time|SetTimerbyFunctionName 0 "FindTarget" (Math|Random|RandomFloatinRange 1e+01 15.0)))
      (Variables|Default|SetFindTargetTimer _returnvalue))))

(event EventTick
  (params (DeltaSeconds :type Float%20%28single-precision%29))
  (if (== (Utilities|Array|Length (Variables|Default|GetTargetList)) 0)
    (bind _outactors (Actor|GetAllActorsOfClass "/Game/Blueprints/PlayerCharacter.PlayerCharacter_C"))
    (bind _output_get (Variables|Default|SetTargetList _outactors))
    (bind _outactors_2 (Actor|GetAllActorsOfClass "/Game/EventStuff/LifeSupport/LifeSupportBP.LifeSupportBP_C"))
    (Utilities|Array|Add _output_get (Utilities|Array|Get(acopy) _outactors_2))
    (bind _outactors_3 (Actor|GetAllActorsOfClass "/Game/EventStuff/Generator/GeneratorBP.GeneratorBP_C"))
    (Variables|Default|SetGeneratorBP (Utilities|Array|Get(acopy) _outactors_3))
    (CallFunction|FindTarget)
    (bind _returnvalue (Utilities|Time|SetTimerbyFunctionName 0 "FindTarget" (Math|Random|RandomFloatinRange 1e+01 15.0)))
    (Variables|Default|SetFindTargetTimer _returnvalue)))

(fn ConstructionScript)

(fn ChaseTarget
  (params (Monster :type Swarm%20Monster%20Object%20Reference))
  (bind _returnvalue (Transformation|GetActorLocation Monster))
  (if (Utilities|Enum|Equal(Enum) (Class|AIController|GetMoveStatus) "Idle")
    (bind _returnvalue_2 (Class|BaseMonster|GetCurrentTarget Monster))
    (bind _returnvalue_3 (AI|Navigation|MovetoActor _returnvalue_2 0.0 true true false))
    (if (Utilities|Enum|Equal(Enum) _returnvalue_3 "Failed")
      (if (AI|Components|NavMovement|IsFalling (Variables|/Script/Engine.Character|GetCharacterMovement Monster))
        (bind _outhit (Collision|LineTraceForObjects _returnvalue (- _returnvalue "0, 0,1000.000000") (Utilities|Array|MakeArray "ObjectTypeQuery1" "ObjectTypeQuery2") false 0 "None"))
        (bind _returnvalue_4 (AI|Navigation|MovetoLocation (.Location (Collision|BreakHitResult _outhit)) 0.0 true true false false))
        (if (Utilities|Enum|Equal(Enum) _returnvalue_4 "Failed")
          (CallFunction|FindTarget :!label _label))
        (else
          (goto _label))))))

(fn CheckValidTarget
  (params (Monster :type Swarm%20Monster%20Object%20Reference))
  (bind (_success _returnvalue) (Class|BaseMonster|GetCurrentTarget Monster))
  (if _success
    (bind _asplayer_character (Utilities|Casting|CastToPlayerCharacter _returnvalue)
      (:then
        (bind _returnvalue_2 (Class|SwarmCharacter|IsAlive _asplayer_character))
        (if _returnvalue_2
          _
          (else
            (CallFunction|FindTarget)
            (Variables|/Script/Swarm.BaseMonster|SetState Monster "EMS_CHASING")))
        (return _returnvalue_2))
      (:CastFailed
        (bind _aslife_support_bp (Utilities|Casting|CastToLifeSupportBP _returnvalue)
          (:then
            (if (<= (Variables|/Game/EventStuff/LifeSupport/LifeSupportBP.LifeSupportBP_C|GetHealth _aslife_support_bp) 0.0)
              (Variables|/Game/Blueprints/AI/SwarmMonster.SwarmMonster_C|SetCanAttack Monster false)
              (Variables|/Script/Swarm.BaseMonster|SetState Monster "EMS_DEAD"))
            (return true))
          (:CastFailed
            _))))
    (else
      (CallFunction|FindTarget)))
  (return _success))

(fn FindTarget
  (bind _asswarm_monster (Utilities|Casting|CastToSwarmMonster (Pawn|GetControlledPawn)))
  (bind _returnvalue (Class|BaseMonster|GetCurrentTarget _asswarm_monster))
  (for _array_element (Variables|Default|GetTargetList)
    (bind _score (CallFunction|ScoreTarget _asswarm_monster _array_element _returnvalue))
    (if (> (+ _score (Math|Random|RandomIntegerinRange -1000 1000)) (LocalVariables|GetBestScore))
      (Variables|/Script/Swarm.BaseMonster|SetTarget _asswarm_monster _array_element)
      (LocalVariables|SetBestScore _score)))
  (Class|KismetSystemLibrary|ClearTimerHandle (Variables|Default|GetFindTargetTimer))
  (bind _returnvalue_2 (Utilities|Time|SetTimerbyFunctionName 0 "FindTarget" (Math|Random|RandomFloatinRange 2e+01 3e+01)))
  (Variables|Default|SetFindTargetTimer _returnvalue_2))

(fn CheckCanAttack
  (params (Monster :type Swarm%20Monster%20Object%20Reference))
  (bind _array_element (Utilities|Array|ForEachLoopwithBreak (Variables|Default|GetTargetList) :!label _label)
    (:LoopBody
      (bind _result (CallFunction|CheckAttackOverlap Monster _array_element))
      (bind _asplayer_character (Utilities|Casting|CastToPlayerCharacter _array_element)
        (:then
          (bind _returnvalue (Class|SwarmCharacter|IsAlive _asplayer_character))
          (if (and _returnvalue (and _result (Variables|/Game/Blueprints/AI/SwarmMonster.SwarmMonster_C|GetCanAttack Monster)))
            (if (Utilities|Enum|Equal(Enum) (Variables|/Script/Swarm.BaseMonster|GetState Monster) "EMS_CHASING") :!label _label_2
              (Variables|/Script/Swarm.BaseMonster|SetTarget Monster _array_element)
              (Variables|/Script/Swarm.BaseMonster|SetState Monster "EMS_ATTACKING")
              (AI|Navigation|StopMovement)
              (Class|KismetSystemLibrary|ClearTimerHandle)
              (bind _returnvalue_2 (Utilities|Time|SetTimerbyFunctionName 0 "FindTarget" (Math|Random|RandomFloatinRange 1e+01 15.0)))
              (Variables|Default|SetFindTargetTimer _returnvalue_2)
              (goto _label Break))
            (else
              (if (Utilities|Enum|Equal(Enum) (Variables|/Script/Swarm.BaseMonster|GetState Monster) "EMS_ATTACKING") :!label _label_3
                (Variables|/Script/Swarm.BaseMonster|SetState Monster "EMS_CHASING")))))
        (:CastFailed
          (if (and _result (Variables|/Game/Blueprints/AI/SwarmMonster.SwarmMonster_C|GetCanAttack Monster))
            (goto _label_2)
            (else
              (goto _label_3))))))))

(fn CheckAttackOverlap
  (params (Monster :type Swarm%20Monster%20Object%20Reference) (Target :type Actor%20Object%20Reference))
  (bind _asplayer_character (Utilities|Casting|CastToPlayerCharacter Target)
    (:then
      (return (Collision|IsOverlappingActor (Variables|/Game/Blueprints/PlayerCharacter.PlayerCharacter_C|GetAttackCollision _asplayer_character) Monster :!class /Script/Engine.PrimitiveComponent)))
    (:CastFailed
      (bind _aslife_support_bp (Utilities|Casting|CastToLifeSupportBP Target)
        (:then
          (return (Collision|IsOverlappingActor (Variables|/Game/EventStuff/LifeSupport/LifeSupportBP.LifeSupportBP_C|GetAttackCollision _aslife_support_bp) Monster :!class /Script/Engine.PrimitiveComponent)))
        (:CastFailed
          (return false))))))

(fn ScoreTarget
  (params (Monster :type Swarm%20Monster%20Object%20Reference) (NewTarget :type Actor%20Object%20Reference) (CurrentTarget :type Actor%20Object%20Reference))
  (bind _asplayer_character (Utilities|Casting|CastToPlayerCharacter NewTarget)
    (:then
      (bind _returnvalue (AI|Navigation|MovetoActor _asplayer_character -1.0 true true false))
      (AI|Navigation|StopMovement)
      (bind _returnvalue_2 (Class|SwarmCharacter|IsAlive _asplayer_character))
      (if (and _returnvalue_2 (not (Utilities|Enum|Equal(Enum) _returnvalue "Failed")))
        (bind _asswarm_player_state (Utilities|Casting|CastToSwarmPlayerState (Variables|/Script/Engine.Pawn|GetPlayerState _asplayer_character))
          (:then
            (bind _output_get (LocalVariables|SetRetScore (+ (- 800 (Math|Float|Truncate (Variables|/Script/Swarm.SwarmCharacter|GetSpeed _asplayer_character))) (Math|Float|Truncate (- 7.8e+03 (Transformation|GetDistanceTo Monster NewTarget))))))
            (if (Variables|/Game/Blueprints/PlayerCharacter.PlayerCharacter_C|GetIsCarryingBattery _asplayer_character)
              (LocalVariables|SetRetScore (+ _output_get 300)))
            (Utilities|IsValid CurrentTarget
              (:Is%20Valid
                (bind _asplayer_character_2 (Utilities|Casting|CastToPlayerCharacter CurrentTarget)
                  (:then
                    (bind _asswarm_player_state_2 (Utilities|Casting|CastToSwarmPlayerState (Variables|/Script/Engine.Pawn|GetPlayerState _asplayer_character_2))
                      (:then
                        (if (<= (+ (Variables|/Script/Swarm.BasePlayerState|GetHealth _asswarm_player_state) 4e+01) (Variables|/Script/Swarm.BasePlayerState|GetHealth _asswarm_player_state_2))
                          (LocalVariables|SetRetScore (+ (LocalVariables|GetRetScore) (* (- 100 (Math|Float|Truncate (Variables|/Script/Swarm.BasePlayerState|GetHealth _asswarm_player_state))) 10))))
                        (return (LocalVariables|GetRetScore)))
                      (:CastFailed
                        _)))
                  (:CastFailed
                    _))
                (return (LocalVariables|GetRetScore)))
              (:Is%20Not%20Valid
                (return (LocalVariables|GetRetScore)))))
          (:CastFailed
            _))
        (else
          (LocalVariables|SetRetScore -10000)))
      (return (LocalVariables|GetRetScore)))
    (:CastFailed
      (if (Variables|/Game/EventStuff/Generator/GeneratorBP.GeneratorBP_C|GetIsPowerOn (Variables|Default|GetGeneratorBP))
        (LocalVariables|SetRetScore (Math|Float|Truncate (- 4.8e+03 (Transformation|GetDistanceTo Monster NewTarget))))
        (elif (== (Math|Random|RandomIntegerinRange 0 5) 0)
          (LocalVariables|SetRetScore 1000)
          (else
            (LocalVariables|SetRetScore 9999999))))
      (return (LocalVariables|GetRetScore)))))