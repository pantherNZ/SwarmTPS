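; Main menu pawn that opens the menu, host and lobby widgets and writes difficulty and modifier choices to the GameInstance.
; It creates a session and opens the map as listen server, or refreshes found sessions every second and joins by server name.
; Returning to the main menu reverses the Host or Find camera sequence, while the forward camera moves are unwired.
; Older SessionHandler and lobby-list code is also left disconnected.
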(event `Host Game`
  (bind _returnvalue (`|CreateWidget` "/Game/Widgets/HostGame_Widget.HostGame_Widget_C"))
  (`UserWidget.AddToViewport` _returnvalue 0)
  (set `self.HostWidget` _returnvalue)
  (set `self.State` "NewEnumerator1"))

(event `self.ReceiveBeginPlay`
  (bind _returnvalue (`|CreateWidget` "/Game/Widgets/Menu_Widget.Menu_Widget_C"))
  (`UserWidget.AddToViewport` _returnvalue 0)
  (set `self.MainWidget` _returnvalue)
  (set `self.State` "NewEnumerator0")
  (bind _asmy_game_instance (cast `/Game/Blueprints/MyGameInstance` (`GameplayStatics.GetGameInstance`)))
  (set `self.GameInstance` _asmy_game_instance)
  (bind _outactors (`GameplayStatics.GetAllActorsOfClass` "/Script/Engine.CameraActor"))
  (for _array_element _outactors
    (bind _returnvalue_2 (`KismetSystemLibrary.GetObjectName` _array_element))
    (if (`KismetStringLibrary.EqualEqual_StrStr` _returnvalue_2 "CameraActor_6")
      (set `self.HostCamera` _array_element)
      (elif (`KismetStringLibrary.EqualEqual_StrStr` _returnvalue_2 "CameraActor_5")
        (set `self.JoinCamera` _array_element)))))

(event `Find Game`
  (bind _returnvalue (`|CreateWidget` "/Game/Widgets/Lobby_Widget.Lobby_Widget_C"))
  (`UserWidget.AddToViewport` _returnvalue 0)
  (set `self.JoinWidget` _returnvalue)
  (set `self.State` "NewEnumerator2")
  (set `self.SearchServers` true)
  (`self.UpdateServerList`)
  (`KismetSystemLibrary.K2_SetTimer` null "UpdateServerList" 1.0 true))

(event `ActivateModifiers`
  (params (Modifiers :type "Array of /Game/Widgets/ModifierType Enum"))
  (set `/Game/Blueprints/MyGameInstance.Modifiers` Modifiers (`self.GameInstance`)))

(event `SetDifficulty`
  (params (Difficulty :type String))
  (bind _gameinstance (`self.GameInstance`))
  (switch `string` Difficulty
    (:`Easy`
      (set `/Game/Blueprints/MyGameInstance.DifficultyMultiplier` 0.5 _gameinstance))
    (:`Normal`
      (set `/Game/Blueprints/MyGameInstance.DifficultyMultiplier` 1.0 _gameinstance))
    (:`hard`
      (set `/Game/Blueprints/MyGameInstance.DifficultyMultiplier` 2.0 _gameinstance))))

(event `Quit`
  (`KismetSystemLibrary.QuitGame` null "Quit"))

(event `Start`
  (params (Players :type Integer) (LAN :type Boolean) (`Server Name` :type String))
  (`CreateSessionCallbackProxy.CreateSession` (`GameplayStatics.GetPlayerController` 0) Players LAN
    (:`OnSuccess`
      (`GameplayStatics.OpenLevel` (`self.Map Name`) true "?listen"))
    (:`OnFailure`
      (`KismetSystemLibrary.PrintString` "CREATE SESSION: FAILED"))))

(event `UpdateServerList`
  (bind _results (`FindSessionsCallbackProxy.FindSessions` (`GameplayStatics.GetPlayerController` 0) 25)
    (:`OnSuccess`
      (set `self.ServerList` _results))))

(event `ReturnToMainMenu`
  (bind _camera (`self.Camera`))
  (bind _camera_2 (`self.Camera`))
  (bind _sequenceplayer (`LevelSequenceActor.SequencePlayer` (`self.JoinGameSequence`)))
  (bind _sequenceplayer_2 (`LevelSequenceActor.SequencePlayer` (`self.HostGameSequence`)))
  (switch `/Game/Blueprints/Menu/Menu` (`self.State`)
    (:`NewEnumerator1`
      (`MovieSceneSequencePlayer.Play` _sequenceplayer_2)
      (`MovieSceneSequencePlayer.ChangePlaybackDirection` _sequenceplayer_2)
      (`PlayerController.SetViewTargetWithBlend` (`GameplayStatics.GetPlayerController` 0) (`self.HostCamera`) 0.0 "VTBlend_Linear" 0.0 false)
      (`SceneComponent.K2_SetWorldLocation` _camera (4743.022461 -10027.061523 596.0) false false)
      (`SceneComponent.K2_SetWorldRotation` _camera (struct :`Yaw` -20.0) false false))
    (:`NewEnumerator2`
      (`MovieSceneSequencePlayer.Play` _sequenceplayer)
      (`MovieSceneSequencePlayer.ChangePlaybackDirection` _sequenceplayer)
      (`PlayerController.SetViewTargetWithBlend` (`GameplayStatics.GetPlayerController` 0) (`self.JoinCamera`) 0.0 "VTBlend_Linear" 0.0 false)
      (`SceneComponent.K2_SetWorldLocation` _camera_2 (4743.022461 -10027.061523 596.0) false false)
      (`SceneComponent.K2_SetWorldRotation` _camera_2 (struct :`Yaw` -20.0) false false))))

(event `Join Game`
  (params (ServerName :type String))
  (for _array_element (`self.ServerList`)
    (if (`KismetStringLibrary.EqualEqual_StrStr` (`FindSessionsCallbackProxy.GetServerName` _array_element) ServerName)
      (`JoinSessionCallbackProxy.JoinSession` (`GameplayStatics.GetPlayerController` 0) _array_element
        (:`OnFailure`
          (`KismetSystemLibrary.PrintString` "JOIN SESSION: FAILED"))))))

(event `self.ReceiveTick`
  (params (DeltaSeconds :type "Float (single-precision)")))

(fn `UserConstructionScript`)