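; Proximity mine Blueprint that explodes when a BaseMonster enters its sphere collision.
; The overlap spawns an explosion particle effect, applies radial damage with falloff that ignores all PlayerCharacter actors, then destroys the mine.
; A short timer, started in ReceiveBeginPlay_Copy, sets a CanStop flag that the overlap logic does not check.
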(event `ReceiveBeginPlay_Copy`
  (`KismetSystemLibrary.K2_SetTimer` null "EnableStop" 0.5))

(event `self.SphereCollision.OnComponentBeginOverlap`
  (params (OtherActor :type "Actor Object Reference") (OtherComp :type "PrimitiveComponent Object Reference") (OtherBodyIndex :type Integer) (bFromSweep :type Boolean) (SweepResult :type "HitResult Structure (by ref)"))
  (bind _returnvalue (`self.K2_GetActorLocation` self))
  (cast `BaseMonster` OtherActor)
  (`GameplayStatics.SpawnEmitterAtLocation` "/Game/StarterContent/Particles/P_Explosion.P_Explosion" (+ _returnvalue 100.0))
  (bind _outactors (`GameplayStatics.GetAllActorsOfClass` "/Game/Blueprints/PlayerCharacter.PlayerCharacter_C"))
  (`GameplayStatics.ApplyRadialDamageWithFalloff` 75.0 0.0 _returnvalue 10.0 300.0 1.0 null _outactors (`self.GetOwner`))
  (`self.K2_DestroyActor`))

(event `self.ReceiveTick`
  (params (DeltaSeconds :type "Float (single-precision)")))

(event `EnableStop`
  (set `self.canStop` true))

(fn `UserConstructionScript`)