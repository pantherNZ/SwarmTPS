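; 3DMoneyDisplay is an actor that shows a floating, fading money popup in the world through a ShowMoney_Widget on its widget component.
; BeginPlay picks a random direction within a narrow upward cone and a random speed, so each popup drifts differently.
; Tick lowers the widget's alpha by FadeSpeed, destroys the actor once fully transparent, and moves it along that direction without sweeping.
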(event `self.ReceiveBeginPlay`
  (set `self.Direction` (`KismetMathLibrary.RandomUnitVectorInCone` (0.0 0.0 1.0) (`KismetMathLibrary.DegreesToRadians` 15.0)))
  (set `self.MoveSpeed` (`KismetMathLibrary.RandomFloatInRange` 75.0 125.0)))

(event `self.ReceiveTick`
  (params (DeltaSeconds :type "Float (single-precision)"))
  (`|ExecutionSequence`
    (:`then_0`
      (bind _asshow_money_widget (cast `/Game/Widgets/ShowMoney_Widget` (`WidgetComponent.GetUserWidgetObject` (`self.Widget`))))
      (bind (_colorandopacity_r _colorandopacity_g _colorandopacity_b _colorandopacity_a) (break `LinearColor` (`UserWidget.ColorAndOpacity` _asshow_money_widget)))
      (bind _returnvalue (- _colorandopacity_a (* DeltaSeconds (`self.FadeSpeed`))))
      (`UserWidget.SetColorAndOpacity` _asshow_money_widget (make `LinearColor` _colorandopacity_r _colorandopacity_g _colorandopacity_b _returnvalue))
      (if (<= _returnvalue 0.0)
        (`self.K2_DestroyActor`)))
    (:`then_1`
      (`self.K2_AddActorWorldOffset` (* (`self.Direction`) (* DeltaSeconds (`self.MoveSpeed`)))))))

(fn `UserConstructionScript`)