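; SwarmGameState is the game state for a wave-based monster game, holding difficulty, the living monster count and the number of players in the vendor.
; On game start the authority copies the difficulty multiplier from the game instance, then both authority and remote start the solar controller and, if that exists, the generator.
; As a stuck-wave failsafe, authority Tick starts a timer when one monster remains, which zeroes the count if still one.
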(event `self.GameStart`
  (`/Engine/EditorBlueprintResources/ActorMacros.Switch Has Authority`
    (:`Authority`
      (bind _asmy_game_instance (cast `/Game/Blueprints/MyGameInstance` (`GameplayStatics.GetGameInstance`)))
      (bind _asswarm_game_state (cast `/Game/Blueprints/SwarmGameState` (`GameplayStatics.GetGameState`)))
      (set `BaseGameState.Difficulty` (`/Game/Blueprints/MyGameInstance.DifficultyMultiplier` _asmy_game_instance) _asswarm_game_state))
    (:`Remote`
      _))
  (bind _outactors (`GameplayStatics.GetAllActorsOfClass` "/Game/EventStuff/SolarPlant/SolarController.SolarController_C"))
  (bind _item (`KismetArrayLibrary.Array_Get` _outactors))
  (`/Engine/EditorBlueprintResources/StandardMacros.IsValid` _item
    (:`Is Valid`
      (`/Game/EventStuff/SolarPlant/SolarController.Start Game` _item)
      (bind _outactors_2 (`GameplayStatics.GetAllActorsOfClass` "/Game/EventStuff/Generator/GeneratorBP.GeneratorBP_C"))
      (bind _item_2 (`KismetArrayLibrary.Array_Get` _outactors_2))
      (`/Engine/EditorBlueprintResources/StandardMacros.IsValid` _item_2
        (:`Is Valid`
          (`/Game/EventStuff/Generator/GeneratorBP.Start` _item_2))
        (:`Is Not Valid`
          (`KismetSystemLibrary.PrintString` "ERROR: Generator BP cannot be found - 'swarmgamestate'"))))
    (:`Is Not Valid`
      (`KismetSystemLibrary.PrintString` "ERROR: Solar panel controller cannot be found - 'swarmgamestate'"))))

(event `self.ReceiveTick`
  (params (DeltaSeconds :type "Float (single-precision)"))
  (`parent.ReceiveTick` DeltaSeconds)
  (`/Engine/EditorBlueprintResources/ActorMacros.Switch Has Authority`
    (:`Authority`
      (if (and (== (`self.MonstersAlive`) 1) (not (`KismetSystemLibrary.K2_IsTimerActiveHandle` (`self.ForceEnd`))))
        (bind _returnvalue (`KismetSystemLibrary.K2_SetTimer` null "ForceEndWave" 15.0))
        (set `self.ForceEnd` _returnvalue)))))

(event `ForceEndWave`
  (if (== (`self.MonstersAlive`) 1)
    (set `self.ForceEnd` (struct))
    (set `self.MonstersAlive` 0)))

(event `AlterPlayerInVendorCount`
  (params (Add :type Integer))
  (set `self.PlayersInVendorCount` (+ Add (`self.PlayersInVendorCount`))))

(fn `UserConstructionScript`)