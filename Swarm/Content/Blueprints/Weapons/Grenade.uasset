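; Grenade projectile that sets an explosion impact particle, shakes nearby cameras on a valid hit and has a limited lifespan.
; Pawn collision turns on shortly after spawn via a timer.
; On the authority, hits that pass CheckIfHit trigger ShakeMulticast at the grenade's location, then destroy it.
; ApplyVelocity forwards launch velocity, gravity scale, max speed and activation state to ApplyMovementMulti, which applies them.
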(event `self.ReceiveBeginPlay`
  ;[1 1 1] Initialisation
  (set `self.ImpactParticle` "/Game/StarterContent/Particles/P_Explosion.P_Explosion")
  (`KismetSystemLibrary.K2_SetTimer` null "Collision" 0.1)
  (`self.SetLifeSpan` 30.0))

(event `Collision`
  ;[1 1 1] Activate Collision With Players
  (`PrimitiveComponent.SetCollisionResponseToChannel` (`self.Projectile`) "ECC_Pawn" "ECR_Block"))

(event `self.Projectile.OnComponentHit`
  (params (OtherActor :type "Actor Object Reference") (OtherComp :type "PrimitiveComponent Object Reference") (NormalImpulse :type "Vector Structure") (Hit :type "HitResult Structure (by ref)"))
  ;[1 1 1] Impact Event
  (`/Engine/EditorBlueprintResources/ActorMacros.Switch Has Authority`
    (:`Authority`
      (bind _returnvalue (`self.CheckIfHit` OtherActor))
      (if _returnvalue
        (`self.ShakeMulticast` (`self.K2_GetActorLocation`))
        (`self.K2_DestroyActor`)))))

(event `ShakeMulticast`
  (params (Location :type "Vector Structure"))
  (`GameplayStatics.PlayWorldCameraShake` "/Game/Blueprints/SwarmCameraShake.SwarmCameraShake_C" Location 0.0 1000.0 0.5))

(event `self.ApplyVelocity`
  (params (VelocityInLocalSpace :type "Vector Structure") (Activate :type Boolean) (GravityScale :type "Float (single-precision)") (ProjectileSpeed :type "Float (single-precision)"))
  (`self.ApplyMovementMulti` VelocityInLocalSpace Activate GravityScale ProjectileSpeed))

(event `ApplyMovementMulti`
  (params (`Velocity Local` :type "Vector Structure") (Activated :type Boolean) (`Gravity Scale` :type "Float (double-precision)") (`Projectile Speed` :type "Float (double-precision)"))
  (bind _movement (`self.Movement`))
  (set `self.Activated` Activated)
  (`ProjectileMovementComponent.SetVelocityInLocalSpace` _movement `Velocity Local`)
  (set `ProjectileMovementComponent.ProjectileGravityScale` `Gravity Scale` _movement)
  (set `ProjectileMovementComponent.MaxSpeed` `Projectile Speed` _movement))

(fn `UserConstructionScript`)