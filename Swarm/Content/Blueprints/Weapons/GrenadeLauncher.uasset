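; Grenade launcher weapon Blueprint that configures an automatic gun firing Grenade projectiles with reduced gravity.
; BeginPlay sets reload time, gun type and ammo on every instance, deriving the total ammo from the clip size.
; After a short delay, only the authority sets projectile, fire timing, weight and explosion and blood particle settings.
; The graph holds only these variable assignments, with no firing logic, and the construction script is empty.
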(event `self.ReceiveBeginPlay`
  (set `self.ReloadTime` 0.967)
  (bind _output_get (set `self.MaxClipAmmo` 6))
  (bind _output_get_2 (set `self.CurrentAmmo` _output_get))
  (set `self.TotalAmmo` (* _output_get_2 40))
  (set `self.GunType` "EGT_GRENADELAUNCHER")
  (`/Engine/EditorBlueprintResources/ActorMacros.Switch Has Authority`
    (:`Authority`
      (`KismetSystemLibrary.Delay` 0.1)
      (set `self.ProjectileClass` "/Game/Blueprints/Weapons/Grenade.Grenade_C")
      (bind _output_get_3 (set `self.ShootTime` 0.633))
      (set `self.BaseShootTime` _output_get_3)
      (set `self.ProjectileSpeed` 30000.0)
      (set `self.ProjectileGravityScale` 0.3)
      (set `self.UseProjectile` true)
      (set `self.IsAutomatic` true)
      (set `self.ParticleTemplates` (`|MakeArray` "/Game/StarterContent/Particles/P_Explosion.P_Explosion" "/Game/Impacts/Particles/P_ImpactBlood.P_ImpactBlood" "/Game/Blood/BloodImpacts/GreenBlood.GreenBlood" "/Game/Blood/BloodImpacts/PurpleBlood.PurpleBlood" :!type "ParticleSystem Object Reference"))
      (set `self.Weight` 7))))

(fn `UserConstructionScript`)