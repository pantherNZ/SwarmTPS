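; Automatic rifle weapon Blueprint that sets its ammo, fire timing, reload, weight and impact particle settings on BeginPlay.
; Its Tracer event runs on the authority, spawning a scaled Bullet actor at the muzzle socket, rotated along the line from the actor to the shot's impact point.
; A random and counter-based tracer throttle is present but disconnected, so every Tracer call on the authority spawns a bullet.
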(event `self.ReceiveBeginPlay`
  (set `self.CurrentAmmo` 30)
  (set `self.MaxClipAmmo` 30)
  (set `self.TotalAmmo` 500)
  (set `self.ParticleTemplates` (`|MakeArray` "/Game/Impacts/Particles/P_ImpactConcrete.P_ImpactConcrete" "/Game/Impacts/Particles/P_ImpactBlood.P_ImpactBlood" "/Game/Blood/BloodImpacts/GreenBlood.GreenBlood" "/Game/Blood/BloodImpacts/PurpleBlood.PurpleBlood" :!type "ParticleSystem Object Reference"))
  (bind _output_get (set `self.ShootTime` 0.2))
  (set `self.BaseShootTime` _output_get)
  (set `self.ReloadTime` 0.967)
  (set `self.IsAutomatic` true)
  (set `self.GunType` "EGT_RIFLE")
  (set `self.Weight` 5))

(event `Tracer`
  (`/Engine/EditorBlueprintResources/ActorMacros.Switch Has Authority`
    (:`Authority`
      (`|SpawnActorFromClass` "/Game/Blueprints/Weapons/Bullet.Bullet_C" (`KismetMathLibrary.MakeTransform` (`SceneComponent.GetSocketLocation` (`self.WeaponMesh`) "Muzzle") (`KismetMathLibrary.FindLookAtRotation` (`self.K2_GetActorLocation`) (`.ImpactPoint` (`GameplayStatics.BreakHitResult` (`self.ShootHitResult`)))) (2.0 2.0 2.0)) "AlwaysSpawn" "OverrideRootScale")
      (set `self.TracerCount` 0))))

(fn `UserConstructionScript`)