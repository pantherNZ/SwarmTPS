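; Firestream is a short-lived projectile weapon actor that expires on its own shortly after spawning.
; ApplyVelocity forwards launch parameters to ApplyMovementMulti, which stores the activation flag and sets the movement component's local velocity, gravity scale and max speed.
; Sphere overlaps destroy it unless the other actor is a SwarmMonster, PlayerCharacter or another Firestream, so it passes through those; no damage is applied here.
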(event `self.ReceiveBeginPlay`
  (`self.SetLifeSpan` 2.0))

(event `self.ApplyVelocity`
  (params (VelocityInLocalSpace :type "Vector Structure") (Activate :type Boolean) (GravityScale :type "Float (single-precision)") (ProjectileSpeed :type "Float (single-precision)"))
  (`self.ApplyMovementMulti` VelocityInLocalSpace Activate GravityScale ProjectileSpeed))

(event `ApplyMovementMulti`
  (params (`Velocity Local` :type "Vector Structure") (Activated :type Boolean) (`Gravity Scale` :type "Float (double-precision)") (`Projectile Speed` :type "Float (double-precision)"))
  (bind _movement (`self.Movement`))
  (set `self.Activated` Activated)
  (`ProjectileMovementComponent.SetVelocityInLocalSpace` _movement `Velocity Local`)
  (set `ProjectileMovementComponent.ProjectileGravityScale` `Gravity Scale` _movement)
  (set `ProjectileMovementComponent.MaxSpeed` `Projectile Speed` _movement))

(event `self.Sphere.OnComponentBeginOverlap`
  (params (OtherActor :type "Actor Object Reference") (OtherComp :type "PrimitiveComponent Object Reference") (OtherBodyIndex :type Integer) (bFromSweep :type Boolean) (SweepResult :type "HitResult Structure (by ref)"))
  (cast `/Game/Blueprints/AI/SwarmMonster` OtherActor
    (:`CastFailed`
      (cast `/Game/Blueprints/PlayerCharacter` OtherActor
        (:`CastFailed`
          (cast `/Game/Blueprints/Weapons/Firestream` OtherActor
            (:`CastFailed`
              (`self.K2_DestroyActor`))))))))

(fn `UserConstructionScript`)