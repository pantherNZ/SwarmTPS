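; Flamethrower weapon Blueprint that configures an automatic gun of the flamethrower type.
; On BeginPlay it sets ammo, fire rate, reload time and weight.
; After a short delay, the authority side alone switches it to projectile firing, using a slow, gravity-free Firestream projectile.
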(event `self.ReceiveBeginPlay`
  (set `self.CurrentAmmo` 50)
  (set `self.MaxClipAmmo` 50)
  (set `self.TotalAmmo` 500)
  (bind _output_get (set `self.ShootTime` 0.05))
  (set `self.BaseShootTime` _output_get)
  (set `self.ReloadTime` 0.967)
  (set `self.IsAutomatic` true)
  (set `self.GunType` "EGT_FLAMETHROWER")
  (set `self.Weight` 7)
  (`/Engine/EditorBlueprintResources/ActorMacros.Switch Has Authority`
    (:`Authority`
      (`KismetSystemLibrary.Delay` 0.1)
      (set `self.ProjectileClass` "/Game/Blueprints/Weapons/Firestream.Firestream_C")
      (set `self.ProjectileSpeed` 500.0)
      (set `self.ProjectileGravityScale` 0.0)
      (set `self.UseProjectile` true))))

(fn `UserConstructionScript`)