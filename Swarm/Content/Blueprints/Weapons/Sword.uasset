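; Melee katana weapon that damages monsters it overlaps while active and can heal its wielder.
; BeginPlay configures it as an automatic melee weapon, and Activate clears the hit list to start a new damage window.
; Server-side overlaps damage each monster once per activation and multicast its hit particle.
; Lifesteal triggers randomly on hits, healing all player characters instead of just the owner when a player-state modifier is present.
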(event `self.ReceiveBeginPlay`
  (set `self.IsAutomatic` true)
  (set `self.IsMelee` true)
  (set `self.GunType` "EGT_KATANA")
  (bind _output_get (set `self.ShootTime` 1.4))
  (set `self.BaseShootTime` _output_get)
  (set `self.ParticleTemplates` (`|MakeArray` "/Game/StarterContent/Particles/P_Explosion.P_Explosion" "/Game/Impacts/Particles/P_ImpactBlood.P_ImpactBlood" :!type "ParticleSystem Object Reference"))
  (set `self.Weight` 3))

(event `self.ReceiveActorBeginOverlap`
  (params (OtherActor :type "Actor Object Reference"))
  (bind (_damage _accuracy _firerate _magazinesize _lifesteal) (break `WeaponStats` (`self.WeaponStats`)))
  (bind _returnvalue (* _damage _lifesteal 0.01))
  (`/Engine/EditorBlueprintResources/ActorMacros.Switch Has Authority`
    (:`Authority`
      (bind _asbase_monster (cast `BaseMonster` OtherActor))
      (if (and (`self.Active`) (not (`KismetArrayLibrary.Array_Contains` (`self.DamagedActors`) _asbase_monster)))
        (`GameplayStatics.ApplyDamage` _asbase_monster _damage null self)
        (`KismetArrayLibrary.Array_Add` (`self.DamagedActors`) _asbase_monster)
        (`self.ImpactMulticast` (`BaseMonster.HitParticle` _asbase_monster))
        (if (and (> _lifesteal 0.0) (`KismetMathLibrary.RandomBool`))
          (bind _asplayer_character (cast `/Game/Blueprints/PlayerCharacter` (`self.GetOwner`)))
          (bind _asswarm_player_state (cast `/Game/Blueprints/SwarmPlayerState` (`Pawn.PlayerState` _asplayer_character)))
          (if (`KismetArrayLibrary.Array_Contains` (`/Game/Blueprints/SwarmPlayerState.Modifiers` _asswarm_player_state) "NewEnumerator3")
            (bind _outactors (`GameplayStatics.GetAllActorsOfClass` "/Game/Blueprints/PlayerCharacter.PlayerCharacter_C"))
            (for _array_element _outactors
              (bind _asplayer_character_2 (cast `/Game/Blueprints/PlayerCharacter` _array_element))
              (`/Game/Blueprints/PlayerCharacter.Lifesteal` _asplayer_character_2 _returnvalue))
            (else
              (`/Game/Blueprints/PlayerCharacter.Lifesteal` _asplayer_character _returnvalue))))))))

(event `ImpactMulticast`
  (params (Impact :type "ParticleSystem Object Reference"))
  (bind _returnvalue (`GameplayStatics.SpawnEmitterAtLocation` Impact (`SceneComponent.K2_GetComponentLocation` (`self.ImpactLocation`))))
  (`SceneComponent.SetWorldScale3D` _returnvalue (3.0 3.0 3.0)))

(fn `Activate`
  (`KismetArrayLibrary.Array_Clear` (`self.DamagedActors`))
  (set `self.Active` true))

(fn `UserConstructionScript`)