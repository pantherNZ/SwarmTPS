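; Pistol weapon that sets its ammo, fire timing, reload, weight, semi-auto mode and impact particle templates on BeginPlay.
; Tracer spawns a scaled Bullet actor on authority, aimed from the actor's location to the shot impact but starting at the muzzle; its random throttle is disconnected.
; Impact audio plays through a server-to-multicast chain, which ImpactSound feeds a zero location, or directly via PlayImpactSound.
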(event `self.ReceiveBeginPlay`
  (set `self.CurrentAmmo` 12)
  (set `self.MaxClipAmmo` 12)
  (set `self.TotalAmmo` 500)
  (set `self.ParticleTemplates` (`|MakeArray` "/Game/Impacts/Particles/P_ImpactConcrete.P_ImpactConcrete" "/Game/Impacts/Particles/P_ImpactBlood.P_ImpactBlood" "/Game/Blood/BloodImpacts/GreenBlood.GreenBlood" "/Game/Blood/BloodImpacts/PurpleBlood.PurpleBlood" :!type "ParticleSystem Object Reference"))
  (bind _output_get (set `self.ShootTime` 0.1))
  (set `self.BaseShootTime` _output_get)
  (set `self.ReloadTime` 1.3)
  (set `self.IsAutomatic` false)
  (set `self.GunType` "EGT_PISTOL")
  (set `self.Weight` 2))

(event `Tracer`
  (`/Engine/EditorBlueprintResources/ActorMacros.Switch Has Authority`
    (:`Authority`
      (`|SpawnActorFromClass` "/Game/Blueprints/Weapons/Bullet.Bullet_C" (`KismetMathLibrary.MakeTransform` (`SceneComponent.GetSocketLocation` (`self.WeaponMesh`) "Muzzle") (`KismetMathLibrary.FindLookAtRotation` (`self.K2_GetActorLocation`) (`.ImpactPoint` (`GameplayStatics.BreakHitResult` (`self.ShootHitResult`)))) (2.0 2.0 2.0)) "AlwaysSpawn" "OverrideRootScale" null null)
      (set `self.TracerCount` 0))))

(event `ImpactSound`
  (`self.Impact Server` (0.0 0.0 0.0)))

(event `Impact Server`
  (params (`Impact Location` :type "Vector Structure"))
  (`self.Impact Multicast` `Impact Location`))

(event `Impact Multicast`
  (params (`Impact Location` :type "Vector Structure"))
  (`GameplayStatics.SpawnSoundAtLocation` "/Game/WeaponSoundsAndFX/Sound/Rifle/Rifle_ImpactBody_Cue.Rifle_ImpactBody_Cue" `Impact Location` (struct) 1.0 1.0 0.0 null null))

(event `self.PlayImpactSound`
  (params (ImpactPosition :type "Vector Structure"))
  (`GameplayStatics.SpawnSoundAtLocation` "/Game/WeaponSoundsAndFX/Sound/Rifle/Rifle_ImpactBody_Cue.Rifle_ImpactBody_Cue" ImpactPosition (struct) 1.0 1.0 0.0 null null))

(fn `UserConstructionScript`)