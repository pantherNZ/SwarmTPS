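; GameHUD is the player's HUD class for a wave-survival game, creating the main HUD, scoreboard and revive widgets and applying saved player options.
; Tick polls the character, player state, game state, generator and life-support building to update the widgets, rebuild lobby lists and detect game over.
; Startup opens name or colour-clash prompts before handing input to the game.
; Functions also handle revive feedback, quit and vendor screens, switching input modes and tracking vendor occupancy.
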(event Custom|CloseMap
  (bind _asswarm_player_state (Utilities|Casting|CastToSwarmPlayerState (Variables|/Script/Engine.Controller|GetPlayerState (Game|Player|GetOwningPlayerController))))
  (bind _createnewname (Default|PlayerNameCheck _asswarm_player_state))
  (if _createnewname
    (CallFunction|CreateChooseNameWidget)
    (else
      (CallFunction|CreateChooseColourWidget))))

(event Custom|ToggleHudControl
  (bind _hudwidget (Variables|Default|GetHUDWidget))
  (bind _playerhealth_widget (Variables|/Game/Widgets/HUD_Widget.HUD_Widget_C|GetPlayerHealth_Widget _hudwidget))
  (bind _mini_map_widget (Variables|/Game/Widgets/HUD_Widget.HUD_Widget_C|GetMini-map_Widget _hudwidget))
  (bind _inventory_widget (Variables|/Game/Widgets/HUD_Widget.HUD_Widget_C|GetInventory_Widget _hudwidget))
  (bind _weaponinfo_widget (Variables|/Game/Widgets/HUD_Widget.HUD_Widget_C|GetWeaponInfo_Widget _hudwidget))
  (bind _powerhud (Variables|/Game/Widgets/HUD_Widget.HUD_Widget_C|GetPowerHUD _hudwidget))
  (if (Variables|Default|GetIsHudControlVisible)
    (Variables|Default|SetIsHudControlVisible false)
    (Default|SetControl _powerhud false)
    (Default|SetControl _playerhealth_widget false)
    (Default|SetControl _mini_map_widget false)
    (Default|SetControl _inventory_widget false)
    (Default|SetControl _weaponinfo_widget false)
    (else
      (Variables|Default|SetIsHudControlVisible true)
      (Default|SetControl _powerhud true)
      (Default|SetControl _playerhealth_widget true)
      (Default|SetControl _mini_map_widget true)
      (Default|SetControl _inventory_widget true)
      (Default|SetControl _weaponinfo_widget true))))

(event Custom|QuitWidgetToggleTimer
  (Variables|Default|SetQuitWidgetOpen false))

(event EventBeginPlay
  (bind _returnvalue (UserInterface|CreateWidget "/Game/Widgets/HUD_Widget.HUD_Widget_C" (Game|Player|GetOwningPlayerController)))
  (UserInterface|Viewport|AddtoViewport _returnvalue 0)
  (Variables|Default|SetHUDWidget _returnvalue)
  (bind _returnvalue_2 (UserInterface|CreateWidget "/Game/Widgets/ScoreBoard_Widget.ScoreBoard_Widget_C" (Game|Player|GetOwningPlayerController)))
  (UserInterface|Viewport|AddtoViewport _returnvalue_2 0)
  (Variables|Default|SetScoreboardWidget _returnvalue_2)
  (bind _returnvalue_3 (UserInterface|CreateWidget "/Game/Widgets/Revival_Widget.Revival_Widget_C" (Game|Player|GetOwningPlayerController)))
  (UserInterface|Viewport|AddtoViewport _returnvalue_3 0)
  (Variables|Default|SetReviveWidget _returnvalue_3)
  (CallFunction|ExecutePlayerOptions)
  (bind _asmy_game_instance (Utilities|Casting|CastToMyGameInstance (Game|GetGameInstance)))
  (Variables|/Script/Engine.PlayerController|SetbShowMouseCursor (Game|Player|GetOwningPlayerController) true)
  (if (.displayhints (Variables|/Game/Blueprints/MyGameInstance.MyGameInstance_C|GetPlayerOptions _asmy_game_instance))
    _
    (else
      _))
  (Utilities|FlowControl|Delay 0.2)
  (CallFunction|CloseMap))

(event EventTick
  (params (DeltaSeconds :type Float%20%28single-precision%29))
  (bind _returnvalue (Game|GetGameState))
  (bind _hudwidget (Variables|Default|GetHUDWidget))
  (bind _hudwidget_2 (Variables|Default|GetHUDWidget))
  (bind _generatorbp (Variables|Default|GetGeneratorBP))
  (bind _lifesupportbp (Variables|Default|GetLifeSupportBP))
  (bind _tooltip (Variables|Default|GetTooltip))
  (bind _playerhealth_widget (Variables|/Game/Widgets/HUD_Widget.HUD_Widget_C|GetPlayerHealth_Widget _hudwidget_2))
  (bind _weaponinfo_widget (Variables|/Game/Widgets/HUD_Widget.HUD_Widget_C|GetWeaponInfo_Widget _hudwidget))
  (bind _tooltip_2 (Variables|/Game/Widgets/HUD_Widget.HUD_Widget_C|GetTooltip _hudwidget))
  (bind _buildinghealthwidget (Variables|/Game/Widgets/HUD_Widget.HUD_Widget_C|GetBuildingHealthWidget _hudwidget))
  (bind _skilldisplay_widget (Variables|/Game/Widgets/PlayerHealth_Widget.PlayerHealth_Widget_C|GetSkillDisplay_Widget _playerhealth_widget))
  (bind _asplayer_character (Utilities|Casting|CastToPlayerCharacter (Game|GetPlayerCharacter 0)))
  (Utilities|IsValid (Variables|/Game/Blueprints/PlayerCharacter.PlayerCharacter_C|GetWeaponSystemController _asplayer_character)
    (:Is%20Valid
      (Utilities|IsValid (Variables|/Script/Swarm.BaseWeaponSystem|GetActiveWeapon (Variables|/Game/Blueprints/PlayerCharacter.PlayerCharacter_C|GetWeaponSystemController _asplayer_character))
        (:Is%20Valid
          (Utilities|IsValid _hudwidget
            (:Is%20Valid
              (Variables|/Game/Widgets/WeaponInfo_Widget.WeaponInfo_Widget_C|SetCurrentAmmo _weaponinfo_widget (Variables|/Script/Swarm.BaseGun|GetCurrentAmmo (Variables|/Script/Swarm.BaseWeaponSystem|GetActiveWeapon (Variables|/Game/Blueprints/PlayerCharacter.PlayerCharacter_C|GetWeaponSystemController _asplayer_character))))
              (Variables|/Game/Widgets/WeaponInfo_Widget.WeaponInfo_Widget_C|SetTotalAmmoVal _weaponinfo_widget (Variables|/Script/Swarm.BaseGun|GetTotalAmmo (Variables|/Script/Swarm.BaseWeaponSystem|GetActiveWeapon (Variables|/Game/Blueprints/PlayerCharacter.PlayerCharacter_C|GetWeaponSystemController _asplayer_character))))
              (bind _asswarm_player_state (Utilities|Casting|CastToSwarmPlayerState (Variables|/Script/Engine.Pawn|GetPlayerState _asplayer_character)))
              (Variables|/Game/Widgets/HUD_Widget.HUD_Widget_C|SetHealth _hudwidget (Variables|/Script/Swarm.BasePlayerState|GetHealth _asswarm_player_state))
              (Variables|/Game/Widgets/HUD_Widget.HUD_Widget_C|SetMoney _hudwidget (Variables|/Script/Swarm.BasePlayerState|GetMoney _asswarm_player_state))
              (Variables|/Game/Widgets/PlayerHealth_Widget.PlayerHealth_Widget_C|SetStamina (Variables|/Game/Widgets/HUD_Widget.HUD_Widget_C|GetPlayerHealth_Widget _hudwidget) (Variables|/Script/Swarm.BasePlayerState|GetStamina _asswarm_player_state))
              (if (Utilities|Enum|Equal(Enum) _tooltip "Insufficient Power")
                (Appearance|SetColorandOpacity _tooltip_2 (Utilities|Struct|MakeSlateColor "(R=1.000000,G=0.000000,B=0.000000,A=1.000000)") :!class /Script/UMG.TextBlock)
                (else
                  (Appearance|SetColorandOpacity _tooltip_2 (Utilities|Struct|MakeSlateColor "(R=0.000000,G=1.000000,B=0.000000,A=1.000000)") :!class /Script/UMG.TextBlock)))
              (Rendering|Components|TextRender|SetText _tooltip_2 (Utilities|Text|ToText(String) _tooltip))
              (bind _asswarm_game_state (Utilities|Casting|CastToSwarmGameState _returnvalue))
              (Variables|/Game/Widgets/HUD_Widget.HUD_Widget_C|SetEnemiesLeft _hudwidget (- (Variables|/Script/Swarm.BaseGameState|GetMonstersMax _asswarm_game_state) (Variables|/Script/Swarm.BaseGameState|GetCurrentWaveKills _asswarm_game_state)))
              (CallFunction|CountPlayers _asswarm_game_state)
              (CallFunction|GameOverCheck)
              (Utilities|FlowControl|Sequence
                (:then_0
                  (if (and (Variables|Default|GetReviving) (Utilities|IsValid _returnvalue))
                    (Variables|/Game/Widgets/Revival_Widget.Revival_Widget_C|SetRecoverPercent (Variables|Default|GetReviveWidget) (Variables|/Script/Swarm.SwarmCharacter|GetReviveProgress (Variables|/Script/Swarm.SwarmCharacter|GetRevivingCharacter _asplayer_character)))))
                (:then_1
                  (if (Variables|Default|GetVendorOpen)
                    _))
                (:then_2
                  (Utilities|IsValid (Variables|/Game/Blueprints/PlayerCharacter.PlayerCharacter_C|GetSkillSystem _asplayer_character)
                    (:Is%20Valid
                      (if (Utilities|Enum|NotEqual(Enum) (Variables|/Script/Swarm.SkillSystem|GetCurrentSkill (Variables|/Game/Blueprints/PlayerCharacter.PlayerCharacter_C|GetSkillSystem _asplayer_character)) (Variables|/Game/Widgets/SkillDisplay_Widget.SkillDisplay_Widget_C|GetSkill _skilldisplay_widget))
                        (Default|UpdateImage _skilldisplay_widget (Variables|/Script/Swarm.SkillSystem|GetCurrentSkill (Variables|/Game/Blueprints/PlayerCharacter.PlayerCharacter_C|GetSkillSystem _asplayer_character)))))))
                (:then_3
                  (Utilities|IsValid _generatorbp
                    (:Is%20Valid
                      (Progress|SetPercent (Variables|/Game/Widgets/PowerHUD_Widget.PowerHUD_Widget_C|GetProgressBar (Variables|/Game/Widgets/HUD_Widget.HUD_Widget_C|GetPowerHUD _hudwidget)) (/ (Variables|/Game/EventStuff/Generator/GeneratorBP.GeneratorBP_C|GetPowerUnits _generatorbp) 1e+03)))
                    (:Is%20Not%20Valid
                      (CallFunction|GetGeneratorRef))))
                (:then_4
                  (if (Variables|Default|GetShowBuildingHealth)
                    (Utilities|IsValid _lifesupportbp
                      (:Is%20Valid
                        (Variables|Default|SetBuildingHealthPercent (/ (Variables|/Game/EventStuff/LifeSupport/LifeSupportBP.LifeSupportBP_C|GetHealth _lifesupportbp) 5e+02))
                        (Widget|SetVisibility _buildinghealthwidget "Visible")
                        (Progress|SetPercent (Variables|/Game/Widgets/BuildingHealth_Widget.BuildingHealth_Widget_C|GetBuildingHealth _buildinghealthwidget) (Variables|Default|GetBuildingHealthPercent)))
                      (:Is%20Not%20Valid
                        (CallFunction|GetLifeSupportRef)))
                    (else
                      (Widget|SetVisibility _buildinghealthwidget "Hidden"))))))))))))

(fn ConstructionScript)

(fn ToggleScoreboard
  (params (On :type Boolean))
  (bind _output_get (Variables|Default|SetScoreboardActive On))
  (Default|Toggle (Variables|Default|GetScoreboardWidget) _output_get))

(fn GameOverCheck
  (if (not (Variables|Default|GetGameOver))
    (bind _asswarm_game_state (Utilities|Casting|CastToSwarmGameState (Game|GetGameState)))
    (if (Utilities|Enum|Equal(Enum) (Variables|/Script/Swarm.BaseGameState|GetGameState _asswarm_game_state) "EGS_GAMEOVER")
      (Variables|Default|SetGameOver true)
      (bind _returnvalue (UserInterface|CreateWidget "/Game/Widgets/EndStats_Widget.EndStats_Widget_C" (Game|GetPlayerController 0)))
      (UserInterface|Viewport|AddtoViewport _returnvalue 0)
      (Input|SetInputModeUIOnly (Game|GetPlayerController 0) _returnvalue "LockAlways"))))

(fn ToggleReviving
  (params (Reviving :type Boolean))
  (bind _revivewidget (Variables|Default|GetReviveWidget))
  (bind _output_get (Variables|Default|SetReviving Reviving))
  (if _output_get
    (bind _returnvalue (Audio|SpawnSound2D "/Game/Sounds/Cues/ReviveCue.ReviveCue" 1.0 1.0 0.0 0))
    (Variables|Default|SetReviveSound _returnvalue)
    (Widget|SetVisibility _revivewidget "Visible")
    (else
      (Utilities|IsValid (Variables|Default|GetReviveSound)
        (:Is%20Valid
          (Audio|Components|Audio|Stop (Variables|Default|GetReviveSound)))
        (:Is%20Not%20Valid
          _))
      (Widget|SetVisibility _revivewidget "Hidden"))))

(fn CountPlayers
  (params (GameState :type Swarm%20Game%20State%20Object%20Reference))
  (bind _playerarray (Variables|/Script/Engine.GameState|GetPlayerArray GameState))
  (bind _returnvalue (Utilities|Array|Length _playerarray))
  (bind _returnvalue_2 (Class|BaseGameState|InLobby GameState))
  (if (and _returnvalue_2 (Utilities|IsValid GameState))
    (if (!= _returnvalue (Variables|Default|GetPlayers))
      (Variables|Default|SetPlayers _returnvalue)
      (bind _asgame_hud (Utilities|Casting|CastToGameHUD (HUD|GetHUD (Game|GetPlayerController 0))))
      (Default|BuildScoreBoard (Variables|GameHUD_C|GetScoreboardWidget _asgame_hud))
      (Default|BuildReadyList (Variables|GameHUD_C|GetHUDWidget _asgame_hud) GameState))))

(fn ProcessQuit
  (bind _returnvalue (Game|Player|GetOwningPlayerController))
  (if (not (Variables|Default|GetQuitWidgetOpen))
    (bind _returnvalue_2 (UserInterface|CreateWidget "/Game/Widgets/Quit_Widget.Quit_Widget_C" _returnvalue))
    (UserInterface|Viewport|AddtoViewport _returnvalue_2 0)
    (Input|SetInputModeUIOnly _returnvalue _returnvalue_2 "DoNotLock")
    (Widget|SetVisibility (Variables|/Game/Widgets/HUD_Widget.HUD_Widget_C|GetCrosshairPanel (Variables|Default|GetHUDWidget)) "Hidden")))

(fn OpenVendor
  (params (Type :type VendorType%20Enum :default "NewEnumerator0"))
  (bind _returnvalue (Game|GetPlayerController 0))
  (switch Utilities|FlowControl|Switch|SwitchonVendorType Type
    (:NewEnumerator0
      (LocalVariables|SetVendor "/Game/Vendor/WeaponVendor/NewWeaponWidget.NewWeaponWidget_C"))
    (:NewEnumerator1
      (LocalVariables|SetVendor "/Game/Vendor/SkillVendor/SkillWidget.SkillWidget_C"))
    (:NewEnumerator2
      (LocalVariables|SetVendor "/Game/Vendor/ItemVendor/ItemsWidget.ItemsWidget_C")))
  (bind _returnvalue_2 (UserInterface|CreateWidget (LocalVariables|GetVendor) _returnvalue))
  (UserInterface|Viewport|AddtoViewport _returnvalue_2 0)
  (Input|SetInputModeUIOnly _returnvalue _returnvalue_2 "LockInFullscreen")
  (Variables|Default|SetVendorOpen true)
  (bind _asswarm_game_state (Utilities|Casting|CastToSwarmGameState (Game|GetGameState)))
  (Default|AlterPlayerinVendorCount _asswarm_game_state 1)
  (Variables|/Script/Engine.PlayerController|SetbShowMouseCursor _returnvalue true))

(fn CreateChooseNameWidget
  (bind _returnvalue (Game|Player|GetOwningPlayerController))
  (bind _returnvalue_2 (UserInterface|CreateWidget "/Game/Widgets/ChooseName_Widget.ChooseName_Widget_C" _returnvalue))
  (UserInterface|Viewport|AddtoViewport _returnvalue_2 0)
  (Input|SetInputModeUIOnly _returnvalue _returnvalue_2 "DoNotLock")
  (Class|Widget|SetUserFocus _returnvalue_2 _returnvalue)
  (Widget|SetKeyboardFocus (Variables|/Game/Widgets/ChooseName_Widget.ChooseName_Widget_C|GetPlayerNameText _returnvalue_2))
  (Class|Widget|SetUserFocus (Variables|/Game/Widgets/ChooseName_Widget.ChooseName_Widget_C|GetPlayerNameText _returnvalue_2) _returnvalue)
  (Variables|/Script/Engine.PlayerController|SetbShowMouseCursor _returnvalue true))

(fn GetGeneratorRef
  (bind _outactors (Actor|GetAllActorsOfClass "/Game/EventStuff/Generator/GeneratorBP.GeneratorBP_C"))
  (Variables|Default|SetGeneratorBP (Utilities|Array|Get(acopy) _outactors)))

(fn GetLifeSupportRef
  (bind _outactors (Actor|GetAllActorsOfClass "/Game/EventStuff/LifeSupport/LifeSupportBP.LifeSupportBP_C"))
  (Variables|Default|SetLifeSupportBP (Utilities|Array|Get(acopy) _outactors)))

(fn ExecutePlayerOptions
  (bind _asmy_game_instance (Utilities|Casting|CastToMyGameInstance (Game|GetGameInstance)))
  (bind _asplayer_character (Utilities|Casting|CastToPlayerCharacter (Game|GetPlayerCharacter 0)))
  (Default|SetColourServer _asplayer_character (.playercolour (Variables|/Game/Blueprints/MyGameInstance.MyGameInstance_C|GetPlayerOptions _asmy_game_instance)))
  (Variables|/Script/Swarm.SwarmCharacter|SetSensitivity _asplayer_character (|(1.250000+(((A*2)-1)*0.750000)) (.gamesensitivity (Variables|/Game/Blueprints/MyGameInstance.MyGameInstance_C|GetPlayerOptions _asmy_game_instance))))
  (Variables|/Game/Blueprints/PlayerCharacter.PlayerCharacter_C|SetZoomModeToggle _asplayer_character (.zoomtoggle (Variables|/Game/Blueprints/MyGameInstance.MyGameInstance_C|GetPlayerOptions _asmy_game_instance))))

(fn CloseVendor
  (Variables|Default|SetVendorOpen false)
  (bind _asswarm_game_state (Utilities|Casting|CastToSwarmGameState (Game|GetGameState)))
  (Default|AlterPlayerinVendorCount _asswarm_game_state -1)
  (bind _asplayer_character (Utilities|Casting|CastToPlayerCharacter (Game|GetPlayerCharacter 0)))
  (Default|RemoveDepenServer _asplayer_character (Variables|Default|GetDependancyType)))

(fn CreateChooseColourWidget
  (bind _returnvalue (Game|Player|GetOwningPlayerController))
  (bind _returnvalue_2 (Game|Player|GetOwningPlayerController))
  (bind _asmy_game_instance (Utilities|Casting|CastToMyGameInstance (Game|GetGameInstance)))
  (bind _outactors (Actor|GetAllActorsOfClass "/Game/Blueprints/PlayerCharacter.PlayerCharacter_C"))
  (bind _array_element (Utilities|Array|ForEachLoopwithBreak _outactors :!label _label)
    (:LoopBody
      (if (!= _array_element (Game|GetPlayerCharacter 0))
        (if (Math|Vector|Equal(Vector) (Math|Conversions|ToVector(LinearColor) (Variables|/Game/Blueprints/PlayerCharacter.PlayerCharacter_C|GetPlayerColour _array_element)) (Math|Conversions|ToVector(LinearColor) (.playercolour (Variables|/Game/Blueprints/MyGameInstance.MyGameInstance_C|GetPlayerOptions _asmy_game_instance))) 0.0001)
          (bind _returnvalue_3 (UserInterface|CreateWidget "/Game/Widgets/ChooseColour_Widget.ChooseColour_Widget_C" _returnvalue_2))
          (UserInterface|Viewport|AddtoViewport _returnvalue_3 0)
          (Input|SetInputModeUIOnly _returnvalue_2 _returnvalue_3 "DoNotLock")
          (Class|Widget|SetUserFocus _returnvalue_3 _returnvalue_2)
          (Variables|/Script/Engine.PlayerController|SetbShowMouseCursor _returnvalue_2 false)
          (LocalVariables|SetCreated true)
          (goto _label Break))))
    (:Completed
      (if (not (LocalVariables|GetCreated))
        (Widget|SetVisibility (Variables|Default|GetHUDWidget) "Visible")
        (Input|SetInputModeGameOnly _returnvalue)
        (Class|WidgetBlueprintLibrary|SetFocustoGameViewport)
        (Variables|/Script/Engine.PlayerController|SetbShowMouseCursor _returnvalue false)))))