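; SwarmPlayerState is the player state for a wave-based swarm game, holding money and the player's name and handling several player-facing UI events.
; A one-time check pushes a saved name through server and local setters, then shows the HUD.
; Saving options rescales the crosshair from the GameInstance setting.
; Wave end shows the ready-up list and switches music off, while other events spawn floating money rewards and short-lived hint icons.
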(event Custom|SetPlayerNameServer
  (params (Name :type String))
  (Class|BasePlayerState|SetGamePlayerName Name))

(event Custom|SavePlayerOptions
  (bind _asmy_game_instance (Utilities|Casting|CastToMyGameInstance (Game|GetGameInstance)))
  (bind _asgame_hud (Utilities|Casting|CastToGameHUD (HUD|GetHUD (Game|GetPlayerController 0))))
  (Variables|/Game/Widgets/WBCrosshair.WBCrosshair_C|Setcrosshair_spread (Variables|/Game/Widgets/HUD_Widget.HUD_Widget_C|GetCrosshairPanel (Variables|/Game/Blueprints/GameHUD.GameHUD_C|GetHUDWidget _asgame_hud)) (* (Variables|/Game/Widgets/WBCrosshair.WBCrosshair_C|GetBase_Spread (Variables|/Game/Widgets/HUD_Widget.HUD_Widget_C|GetCrosshairPanel (Variables|/Game/Blueprints/GameHUD.GameHUD_C|GetHUDWidget _asgame_hud))) (|(1.250000+(((A*2)-1)*0.750000)) (.crosshairscale (Variables|/Game/Blueprints/MyGameInstance.MyGameInstance_C|GetPlayerOptions _asmy_game_instance)))))
  (Variables|/Game/Widgets/WBCrosshair.WBCrosshair_C|Setcrosshair_length (Variables|/Game/Widgets/HUD_Widget.HUD_Widget_C|GetCrosshairPanel (Variables|/Game/Blueprints/GameHUD.GameHUD_C|GetHUDWidget _asgame_hud)) (* (Variables|/Game/Widgets/WBCrosshair.WBCrosshair_C|GetBase_Length (Variables|/Game/Widgets/HUD_Widget.HUD_Widget_C|GetCrosshairPanel (Variables|/Game/Blueprints/GameHUD.GameHUD_C|GetHUDWidget _asgame_hud))) (|(1.250000+(((A*2)-1)*0.750000)) (.crosshairscale (Variables|/Game/Blueprints/MyGameInstance.MyGameInstance_C|GetPlayerOptions _asmy_game_instance))))))

(event Custom|Create%20Hint%20Icon
  (params (World%20Location :type Vector) (Owner :type Player%20Character%20Object%20Reference))
  (bind _returnvalue (Game|SpawnActorfromClass "/Game/Blueprints/Hint/HintAlert.HintAlert_C" (Math|Transform|MakeTransform World%20Location) "AlwaysSpawn" Owner 0))
  (Actor|SetLifeSpan _returnvalue 1e+01))

(event Custom|SetPlayerName
  (params (Name :type String))
  (CallFunction|SetPlayerNameServer Name)
  (Networking|SwitchHasAuthority
    (:Remote
      (Class|BasePlayerState|SetGamePlayerName Name))))

(event Custom|DisplayMoneyReward
  (params (Val :type Float%20%28single-precision%29) (Location :type Vector))
  (bind _returnvalue (Game|SpawnActorfromClass "/Game/Blueprints/3DMoneyDisplay.3DMoneyDisplay_C" (Math|Transform|MakeTransform Location) "AlwaysSpawn" (Game|GetPlayerController 0) 0))
  (bind _asshow_money_widget (Utilities|Casting|CastToShowMoney_Widget (UserInterface|GetUserWidgetObject (Variables|/Game/Blueprints/3DMoneyDisplay.3DMoneyDisplay_C|GetWidget _returnvalue))))
  (Rendering|Components|TextRender|SetText (Variables|/Game/Widgets/ShowMoney_Widget.ShowMoney_Widget_C|GetTextBlock _asshow_money_widget) (Utilities|Text|ToText(String) (Utilities|String|ToString(Integer) (Math|Float|Round Val)))))

(event EventWaveEnd
  (bind _asgame_hud (Utilities|Casting|CastToGameHUD (HUD|GetHUD (Game|GetPlayerController 0))))
  (bind _asswarm_game_state (Utilities|Casting|CastToSwarmGameState (Game|GetGameState)))
  (Widget|SetVisibility (Variables|/Game/Widgets/HUD_Widget.HUD_Widget_C|GetReadyUpPanel (Variables|/Game/Blueprints/GameHUD.GameHUD_C|GetHUDWidget _asgame_hud)) "Visible")
  (Default|BuildReadyList (Variables|/Game/Blueprints/GameHUD.GameHUD_C|GetHUDWidget _asgame_hud) _asswarm_game_state)
  (bind _asplayer_character (Utilities|Casting|CastToPlayerCharacter (Game|GetPlayerCharacter 0)))
  (Default|CallMusic _asplayer_character false))

(event EventShowMoneyonHUD
  (params (Val :type Float%20%28single-precision%29) (Location :type Vector :default "0, 0, 0"))
  (CallFunction|DisplayMoneyReward Val Location))

(event EventBeginPlay
  (Variables|Default|SetMoney 60345))

(fn ConstructionScript)

(fn PlayerNameCheck
  (bind _returnvalue (Game|GetPlayerController 0))
  (Utilities|FlowControl|DoOnce false
    (:Completed
      (bind _asmy_game_instance (Utilities|Casting|CastToMyGameInstance (Game|GetGameInstance)))
      (if (Utilities|Enum|Equal(Enum) (.playername (Variables|/Game/Blueprints/MyGameInstance.MyGameInstance_C|GetPlayerOptions _asmy_game_instance)) "Unnamed")
        (return true)
        (else
          (CallFunction|SetPlayerName (.playername (Variables|/Game/Blueprints/MyGameInstance.MyGameInstance_C|GetPlayerOptions _asmy_game_instance)))
          (Input|SetInputModeGameOnly _returnvalue)
          (Class|WidgetBlueprintLibrary|SetFocustoGameViewport)
          (bind _asgame_hud (Utilities|Casting|CastToGameHUD (HUD|GetHUD _returnvalue)))
          (Widget|SetVisibility (Variables|/Game/Blueprints/GameHUD.GameHUD_C|GetHUDWidget _asgame_hud) "Visible")
          (return false))))))